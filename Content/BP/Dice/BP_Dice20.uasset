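; BP_Dice20 is a twenty-sided die that reports a score for the face pointing up.
; GetSideUp loops through per-face Box components, picks the first whose world roll and pitch are near zero, and returns its number times the point multiplier, rounded.
; Sphere overlaps with BP_ScoreMultiplier actors set that multiplier, and leaving one resets it.
; Random material code in the construction script is disconnected.
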(event `self.Sphere.OnComponentBeginOverlap`
  (params (OverlappedComponent :type "PrimitiveComponent Object Reference") (OtherActor :type "Actor Object Reference") (OtherComp :type "PrimitiveComponent Object Reference") (OtherBodyIndex :type Integer) (bFromSweep :type Boolean) (SweepResult :type "HitResult Structure (by ref)"))
  ;[1 1 1] Setting Point Multiplier
  (if (== (`GameplayStatics.GetObjectClass` OtherActor) "/Game/BP/Table/BP_ScoreMultiplier.BP_ScoreMultiplier_C")
    (set `self.PointMultiplierValue` (`/Game/BP/Table/BP_ScoreMultiplier.PointMultiplierValue` (cast `/Game/BP/Table/BP_ScoreMultiplier` OtherActor :!pure true)))))

(event `self.Sphere.OnComponentEndOverlap`
  (params (OverlappedComponent :type "PrimitiveComponent Object Reference") (OtherActor :type "Actor Object Reference") (OtherComp :type "PrimitiveComponent Object Reference") (OtherBodyIndex :type Integer))
  ;[1 1 1] Setting Point Multiplier
  (if (== (`GameplayStatics.GetObjectClass` OtherActor) "/Game/BP/Table/BP_ScoreMultiplier.BP_ScoreMultiplier_C")
    (set `self.PointMultiplierValue` 1.0)))

(fn `GetSideUp`
  (returns (DiceValue :type Integer))
  (bind (_returnvalue_roll _returnvalue_pitch) (`KismetMathLibrary.BreakRotator` (`SceneComponent.K2_GetComponentRotation` (`self.BoxCheck`))))
  (for _index (range (`self.NumOfSides`))
    (switch `int` _index
      (:`Default`
        (set `self.BoxCheck` (`self.Box1`) :!label _label))
      (:`0`
        (goto _label))
      (:`1`
        (set `self.BoxCheck` (`self.Box2`)))
      (:`2`
        (set `self.BoxCheck` (`self.Box3`)))
      (:`3`
        (set `self.BoxCheck` (`self.Box4`)))
      (:`4`
        (set `self.BoxCheck` (`self.Box5`)))
      (:`5`
        (set `self.BoxCheck` (`self.Box6`)))
      (:`6`
        (set `self.BoxCheck` (`self.Box7`)))
      (:`7`
        (set `self.BoxCheck` (`self.Box8`)))
      (:`8`
        (set `self.BoxCheck` (`self.Box9`)))
      (:`9`
        (set `self.BoxCheck` (`self.Box10`)))
      (:`10`
        (set `self.BoxCheck` (`self.Box11`)))
      (:`11`
        (set `self.BoxCheck` (`self.Box12`)))
      (:`12`
        (set `self.BoxCheck` (`self.Box13`)))
      (:`13`
        (set `self.BoxCheck` (`self.Box14`)))
      (:`14`
        (set `self.BoxCheck` (`self.Box15`)))
      (:`15`
        (set `self.BoxCheck` (`self.Box16`)))
      (:`16`
        (set `self.BoxCheck` (`self.Box17`)))
      (:`17`
        (set `self.BoxCheck` (`self.Box18`)))
      (:`18`
        (set `self.BoxCheck` (`self.Box19`)))
      (:`19`
        (set `self.BoxCheck` (`self.Box20`))))
    (if (`KismetMathLibrary.NearlyEqual_FloatFloat` _returnvalue_roll 0.0 25.0)
      (if (`KismetMathLibrary.NearlyEqual_FloatFloat` _returnvalue_pitch 0.0 25.0)
        (bind _output_get (set `self.DiceValue` (+ _index 1)))
        (return (`KismetMathLibrary.Round` (* _output_get (`self.PointMultiplierValue`))))))))

(fn `UserConstructionScript`)