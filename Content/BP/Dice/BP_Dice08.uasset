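; BP_Dice08 is an eight-sided die that reports a score for the face pointing up.
; GetSideUp loops over per-face box components, picks the first with world roll and pitch near zero within a loose tolerance, and returns its number times the point multiplier.
; The Sphere takes that multiplier from an overlapped BP_ScoreMultiplier and resets it to one on exit.
; Random material code in the construction script is disconnected.
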(event `self.Sphere.OnComponentBeginOverlap`
  (params (OverlappedComponent :type "PrimitiveComponent Object Reference") (OtherActor :type "Actor Object Reference") (OtherComp :type "PrimitiveComponent Object Reference") (OtherBodyIndex :type Integer) (bFromSweep :type Boolean) (SweepResult :type "HitResult Structure (by ref)"))
  ;[1 1 1] Setting Point Multiplier
  (if (== (`GameplayStatics.GetObjectClass` OtherActor) "/Game/BP/Table/BP_ScoreMultiplier.BP_ScoreMultiplier_C")
    (set `self.PointMultiplierValue` (`/Game/BP/Table/BP_ScoreMultiplier.PointMultiplierValue` (cast `/Game/BP/Table/BP_ScoreMultiplier` OtherActor :!pure true)))))

(event `self.Sphere.OnComponentEndOverlap`
  (params (OverlappedComponent :type "PrimitiveComponent Object Reference") (OtherActor :type "Actor Object Reference") (OtherComp :type "PrimitiveComponent Object Reference") (OtherBodyIndex :type Integer))
  ;[1 1 1] Setting Point Multiplier
  (if (== (`GameplayStatics.GetObjectClass` OtherActor) "/Game/BP/Table/BP_ScoreMultiplier.BP_ScoreMultiplier_C")
    (set `self.PointMultiplierValue` 1)))

(fn `GetSideUp`
  (returns (DiceValue :type Integer))
  (bind (_returnvalue_roll _returnvalue_pitch) (`KismetMathLibrary.BreakRotator` (`SceneComponent.K2_GetComponentRotation` (`self.BoxCheck`))))
  (for _index (range (`self.NumOfSides`))
    (switch `int` _index
      (:`Default`
        (set `self.BoxCheck` (`self.Box1`) :!label _label))
      (:`0`
        (goto _label))
      (:`1`
        (set `self.BoxCheck` (`self.Box2`)))
      (:`2`
        (set `self.BoxCheck` (`self.Box3`)))
      (:`3`
        (set `self.BoxCheck` (`self.Box4`)))
      (:`4`
        (set `self.BoxCheck` (`self.Box5`)))
      (:`5`
        (set `self.BoxCheck` (`self.Box6`)))
      (:`6`
        (set `self.BoxCheck` (`self.Box7`)))
      (:`7`
        (set `self.BoxCheck` (`self.Box8`))))
    (if (`KismetMathLibrary.NearlyEqual_FloatFloat` _returnvalue_roll 0.0 50.0)
      (if (`KismetMathLibrary.NearlyEqual_FloatFloat` _returnvalue_pitch 0.0 50.0)
        (bind _output_get (set `self.DiceValue` (+ _index 1)))
        (return (* _output_get (`self.PointMultiplierValue`)))))))

(fn `UserConstructionScript`)