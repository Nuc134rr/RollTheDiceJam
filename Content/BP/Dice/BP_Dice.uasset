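; BP_Dice is a die Blueprint that reports which of its faces is pointing up.
; GetSideUp loops over the side count, mapping each index to one of six Box components that serve as face markers.
; The first box with world roll and pitch both near zero, within a loose tolerance, sets and returns DiceValue as its one-based index.
; Detection relies purely on component orientation, without traces.
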(fn `GetSideUp`
  (returns (DiceValue :type Integer))
  (bind (_returnvalue_roll _returnvalue_pitch) (`KismetMathLibrary.BreakRotator` (`SceneComponent.K2_GetComponentRotation` (`self.BoxCheck`))))
  (for _index (range (`self.NumOfSides`))
    (switch `int` _index
      (:`Default`
        (set `self.BoxCheck` (`self.Box1`) :!label _label))
      (:`0`
        (goto _label))
      (:`1`
        (set `self.BoxCheck` (`self.Box2`)))
      (:`2`
        (set `self.BoxCheck` (`self.Box3`)))
      (:`3`
        (set `self.BoxCheck` (`self.Box4`)))
      (:`4`
        (set `self.BoxCheck` (`self.Box5`)))
      (:`5`
        (set `self.BoxCheck` (`self.Box6`))))
    (if (`KismetMathLibrary.NearlyEqual_FloatFloat` _returnvalue_roll 0.0 25.0)
      (if (`KismetMathLibrary.NearlyEqual_FloatFloat` _returnvalue_pitch 0.0 25.0)
        (bind _output_get (set `self.DiceValue` (+ _index 1)))
        (return _output_get)))))

(fn `UserConstructionScript`)