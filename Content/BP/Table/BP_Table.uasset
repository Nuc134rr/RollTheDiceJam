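; BP_Table is a table actor that scatters a random number of score multiplier actors across its Plane component.
; BeginPlay spawns the set, and BeginTurn destroys the tracked multipliers and spawns a fresh set.
; Each spawn location is a random point within the plane's bounds, re-rolled until a small sphere trace on the Visibility channel finds no hit, with no retry limit.
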(event `self.ReceiveBeginPlay`
  (set `self.NumberOfDots` (`KismetMathLibrary.RandomIntegerInRange` 0 9) :!label _label)
  (for _ (range (+ (`self.NumberOfDots`) 1))
    (bind _returnvalue (`self.CheckForOverlappingDots`))
    (bind _returnvalue_2 (`|SpawnActorFromClass` "/Game/BP/Table/BP_ScoreMultiplier.BP_ScoreMultiplier_C" (`KismetMathLibrary.MakeTransform` _returnvalue) "Undefined" "OverrideRootScale" null null))
    (`KismetArrayLibrary.Array_Add` (`self.ScoreMultiplier`) _returnvalue_2)))

(event `BeginTurn`
  (bind _scoremultiplier (`self.ScoreMultiplier`))
  (for _array_element _scoremultiplier
    (`self.K2_DestroyActor` _array_element))
  (`KismetArrayLibrary.Array_Clear` _scoremultiplier)
  (goto _label))

(fn `CheckForOverlappingDots`
  (returns (ReturnValue :type "Vector Structure"))
  (bind _output_get (set `self.RandomPoint` (`self.GetPointOnPlane`) :!label _label))
  (bind (_outhit _returnvalue) (`KismetSystemLibrary.SphereTraceSingle` _output_get _output_get 20.0 "TraceTypeQuery1"))
  (if _returnvalue
    (goto _label)
    (else
      (return _output_get))))

(fn `GetPointOnPlane`
  (returns (ReturnValue :type "Vector Structure"))
  (bind (_origin _boxextent) (`KismetSystemLibrary.GetComponentBounds` (`self.Plane`)))
  (return (`KismetMathLibrary.RandomPointInBoundingBox` _origin _boxextent)))

(fn `UserConstructionScript`)